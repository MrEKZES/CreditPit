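; Gambling machine actor that earns the player money when an NPC enters its box trigger.
; NPC overlap marks it busy and loops over that NPC's RollCount, aiming to add BetSum to the third-person character's Money after each timed roll.
; The Delay sits inside the loop, so repeat calls do not queue separate waits.
; Any end overlap clears IsBusy; the character reference is never assigned here.
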(event OnComponentBeginOverlap(Box)
  (params (OverlappedComponent :type Primitive%20Component%20Object%20Reference) (OtherActor :type Actor%20Object%20Reference) (OtherComp :type Primitive%20Component%20Object%20Reference) (OtherBodyIndex :type Integer) (bFromSweep :type Boolean) (SweepResult :type Hit%20Result%20Structure%20%28by%20ref%29))
  (bind _as_bp_thirdpersoncharacter (Variables|Default|GetAs%20BP_ThirdPersonCharacter))
  (bind _asbp_npc (Utilities|Casting|CastToBP_NPC OtherActor))
  (bind _output_get (Variables|Default|SetAs%20BP%20NPC _asbp_npc))
  (Variables|GamblingMachine|SetbIsBusy true)
  (for _index (range 0 (Variables|/Game/Project/Blueprints/Actors/NPC/BP_NPC.BP_NPC_C|GetRollCount _output_get))
    (Utilities|FlowControl|Delay (Variables|GamblingMachine|GetTimeBetwenRoll))
    (Variables|/Game/ThirdPerson/Blueprints/BP_ThirdPersonCharacter.BP_ThirdPersonCharacter_C|SetMoney _as_bp_thirdpersoncharacter (+ (Variables|/Game/ThirdPerson/Blueprints/BP_ThirdPersonCharacter.BP_ThirdPersonCharacter_C|GetMoney _as_bp_thirdpersoncharacter) (Variables|/Game/Project/Blueprints/Actors/NPC/BP_NPC.BP_NPC_C|GetBetSum _output_get)))))

(event OnComponentEndOverlap(Box)
  (params (OverlappedComponent :type Primitive%20Component%20Object%20Reference) (OtherActor :type Actor%20Object%20Reference) (OtherComp :type Primitive%20Component%20Object%20Reference) (OtherBodyIndex :type Integer))
  (Variables|GamblingMachine|SetbIsBusy false))

(event EventBeginPlay)

(event Collision|EventActorBeginOverlap
  (params (OtherActor :type Actor%20Object%20Reference)))

(event EventTick
  (params (DeltaSeconds :type Float%20%28single-precision%29)))

(fn ConstructionScript)