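; Tutorial spawner actor that scripts the Chapter 1 intro dialog: a debt collector threatens the player, then points to the wall lever to start work.
; BeginPlay caches the main-level HUD, and PlayChapter1 queues lines through a macro that waits out the current dialog window's delay before adding the next.
; The HUD's WidgetMayBeCreate flag is off during the sequence.
; Nothing in this Blueprint triggers PlayChapter1; its only call is disconnected.
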(event Custom|PlayChapter1
  (Variables|/Game/Project/Blueprints/UI/HUDs/MainLevels/BP_HUDMainLevels.BP_HUDMainLevels_C|SetbWidgetMayBeCreate (Variables|Default|GetAs%20BP%20HUDMain%20Levels) false)
  (Utilities|NewDialogWindowwithDelay "Hello" 1)
  (Utilities|NewDialogWindowwithDelay "Короче ты мне задолжал и много" 2)
  (Utilities|NewDialogWindowwithDelay "Не вернёшь долг я тебя на куски порублю" 3)
  (Utilities|NewDialogWindowwithDelay "Я отдал тебе не развитый отдел казика, это последний раз когда я тебе верю" 5)
  (Utilities|NewDialogWindowwithDelay "Чтобы начать работать нажми на рычаг на стене" 3)
  (Variables|/Game/Project/Blueprints/UI/HUDs/MainLevels/BP_HUDMainLevels.BP_HUDMainLevels_C|SetbWidgetMayBeCreate (Variables|Default|GetAs%20BP%20HUDMain%20Levels) true))

(event EventBeginPlay
  (bind _asbp_hudmain_levels (Utilities|Casting|CastToBP_HUDMainLevels (HUD|GetHUD (Game|GetPlayerController 0))))
  (Variables|Default|SetAs%20BP%20HUDMain%20Levels _asbp_hudmain_levels))

(fn ConstructionScript)

(fn PreInteract
  (return ""))