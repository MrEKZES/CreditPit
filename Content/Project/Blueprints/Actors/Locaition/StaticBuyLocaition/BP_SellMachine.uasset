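; BP_SellMachine is an interactable actor that opens a purchase widget for a casino game location.
; It caches the main-level HUD on BeginPlay, then Interact switches on LocaitionType to add the matching gambling machine, poker or blackjack buy widget, passing itself along.
; PreInteract supplies the key prompt text for interaction.
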(event EventBeginPlay
  (bind _asbp_hudmain_levels (Utilities|Casting|CastToBP_HUDMainLevels (HUD|GetHUD (Game|GetPlayerController 0))))
  (Variables|Default|SetAs%20BP%20HUDMain%20Levels _asbp_hudmain_levels))

(event EventInteract
  (switch Utilities|FlowControl|Switch|SwitchonE_TypeOfPlatform (Variables|Default|GetLocaitionType)
    (:NewEnumerator0
      (Default|AddWBPBuyGamblingMachine (Variables|Default|GetAs%20BP%20HUDMain%20Levels) self))
    (:NewEnumerator1
      (Default|AddWBPBuyPoker (Variables|Default|GetAs%20BP%20HUDMain%20Levels) self))
    (:NewEnumerator2
      (Default|AddWBPBuyBlackJack (Variables|Default|GetAs%20BP%20HUDMain%20Levels) self))))

(fn ConstructionScript)

(fn PreInteract
  (return "Press E to interact"))