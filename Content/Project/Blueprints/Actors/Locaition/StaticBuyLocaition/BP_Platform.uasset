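; Room platform tile that hosts a sell machine and two doors, giving the machine its location type and spawn points.
; On BeginPlay it sets each door's room spawn location 800 units away along -X or -Y.
; Overlap triggers remove doors and dividing walls on adjoining platforms and store left, right and bottom neighbour links.
; Player entry hides its dividing walls and selected neighbour walls; exit restores only its own.
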(event OnComponentBeginOverlap(ButtomPlatfromTriger)
  (params (OverlappedComponent :type Primitive%20Component%20Object%20Reference) (OtherActor :type Actor%20Object%20Reference) (OtherComp :type Primitive%20Component%20Object%20Reference) (OtherBodyIndex :type Integer) (bFromSweep :type Boolean) (SweepResult :type Hit%20Result%20Structure%20%28by%20ref%29))
  ;[0.15 0.15 0.15 0.5] Set platforms link
  (bind _asbp_platform (Utilities|Casting|CastToBP_Platform OtherActor)
    (:then
      (Variables|Default|SetButtomPlatform _asbp_platform))
    (:CastFailed
      (bind _asbp_platform_admin (Utilities|Casting|CastToBP_PlatformAdmin OtherActor))
      (Variables|Default|SetButtomPlatformAdmin _asbp_platform_admin))))

(event OnComponentBeginOverlap(PlayerTrigger)
  (params (OverlappedComponent :type Primitive%20Component%20Object%20Reference) (OtherActor :type Actor%20Object%20Reference) (OtherComp :type Primitive%20Component%20Object%20Reference) (OtherBodyIndex :type Integer) (bFromSweep :type Boolean) (SweepResult :type Hit%20Result%20Structure%20%28by%20ref%29))
  (bind _leftplatform (Variables|Default|GetLeftPlatform))
  (bind _rightplatform (Variables|Default|GetRightPlatform))
  (bind _buttomplatform (Variables|Default|GetButtomPlatform))
  ;[0.15 0.15 0.15 0.5] Player triggers
  (Utilities|Casting|CastToBP_ThirdPersonCharacter OtherActor)
  (CallFunction|SetNewVisibilitywithValidCorection false (Variables|Default|GetDWallY))
  (CallFunction|SetNewVisibilitywithValidCorection false (Variables|Default|GetDWallX))
  (Utilities|FlowControl|DoOnce false :!label _label
    (:Completed
      (Utilities|IsValid _leftplatform
        (:Is%20Valid
          (CallFunction|SetNewVisibilitywithValidCorection _leftplatform false (Variables|BP_Platform_C|GetWallY _leftplatform))
          (CallFunction|SetNewVisibilitywithValidCorection _leftplatform false (Variables|BP_Platform_C|GetDWallX _leftplatform)))
        (:Is%20Not%20Valid
          _))
      (Utilities|IsValid _rightplatform
        (:Is%20Valid
          (CallFunction|SetNewVisibilitywithValidCorection _rightplatform false (Variables|BP_Platform_C|GetWallX _rightplatform))
          (CallFunction|SetNewVisibilitywithValidCorection _rightplatform false (Variables|BP_Platform_C|GetDWallY _rightplatform)))
        (:Is%20Not%20Valid
          _))
      (Utilities|IsValid _buttomplatform
        (:Is%20Valid
          (CallFunction|SetNewVisibilitywithValidCorection _buttomplatform false (Variables|BP_Platform_C|GetWallX _buttomplatform))
          (CallFunction|SetNewVisibilitywithValidCorection _buttomplatform false (Variables|BP_Platform_C|GetWallY _buttomplatform)))
        (:Is%20Not%20Valid
          _))
      (Utilities|FlowControl|Delay 0.2)
      (goto _label Reset))))

(event OnComponentEndOverlap(PlayerTrigger)
  (params (OverlappedComponent :type Primitive%20Component%20Object%20Reference) (OtherActor :type Actor%20Object%20Reference) (OtherComp :type Primitive%20Component%20Object%20Reference) (OtherBodyIndex :type Integer))
  ;[0.15 0.15 0.15 0.5] Player triggers
  (Utilities|Casting|CastToBP_ThirdPersonCharacter OtherActor)
  (CallFunction|SetNewVisibilitywithValidCorection true (Variables|Default|GetDWallY))
  (CallFunction|SetNewVisibilitywithValidCorection true (Variables|Default|GetDWallX)))

(event OnComponentBeginOverlap(TriggerDoorX)
  (params (OverlappedComponent :type Primitive%20Component%20Object%20Reference) (OtherActor :type Actor%20Object%20Reference) (OtherComp :type Primitive%20Component%20Object%20Reference) (OtherBodyIndex :type Integer) (bFromSweep :type Boolean) (SweepResult :type Hit%20Result%20Structure%20%28by%20ref%29))
  ;[0.15 0.15 0.15 0.5] Destroy Door system if room has already been created
  (bind _asbp_platform (Utilities|Casting|CastToBP_Platform OtherActor))
  (for _array_element (Actor|GetComponentsByClass _asbp_platform "/Script/Engine.ActorComponent")
    (if (Utilities|Enum|Equal(Enum) (Utilities|GetObjectName _array_element) "BP_DoorX")
      (CallFunction|DestroyDoorX _asbp_platform))))

(event OnComponentBeginOverlap(TriggerDoorY)
  (params (OverlappedComponent :type Primitive%20Component%20Object%20Reference) (OtherActor :type Actor%20Object%20Reference) (OtherComp :type Primitive%20Component%20Object%20Reference) (OtherBodyIndex :type Integer) (bFromSweep :type Boolean) (SweepResult :type Hit%20Result%20Structure%20%28by%20ref%29))
  ;[0.15 0.15 0.15 0.5] Destroy Door system if room has already been created
  (bind _asbp_platform (Utilities|Casting|CastToBP_Platform OtherActor))
  (for _array_element (Actor|GetComponentsByClass _asbp_platform "/Script/Engine.ActorComponent")
    (if (Utilities|Enum|Equal(Enum) (Utilities|GetObjectName _array_element) "BP_DoorY")
      (CallFunction|DestroyDoorY _asbp_platform))))

(event OnComponentBeginOverlap(TriggerDwallX)
  (params (OverlappedComponent :type Primitive%20Component%20Object%20Reference) (OtherActor :type Actor%20Object%20Reference) (OtherComp :type Primitive%20Component%20Object%20Reference) (OtherBodyIndex :type Integer) (bFromSweep :type Boolean) (SweepResult :type Hit%20Result%20Structure%20%28by%20ref%29))
  ;[0.15 0.15 0.15 0.5] Destroy DWalls if room has already created
  (bind _asbp_platform (Utilities|Casting|CastToBP_Platform OtherActor))
  (for _array_element (Actor|GetComponentsByClass _asbp_platform "/Script/Engine.ActorComponent")
    (if (Utilities|Enum|Equal(Enum) (Utilities|GetObjectName _array_element) "DWallX")
      (CallFunction|DestroyDWallX _asbp_platform))))

(event OnComponentBeginOverlap(TriggerDWallY)
  (params (OverlappedComponent :type Primitive%20Component%20Object%20Reference) (OtherActor :type Actor%20Object%20Reference) (OtherComp :type Primitive%20Component%20Object%20Reference) (OtherBodyIndex :type Integer) (bFromSweep :type Boolean) (SweepResult :type Hit%20Result%20Structure%20%28by%20ref%29))
  ;[0.15 0.15 0.15 0.5] Destroy DWalls if room has already created
  (bind _asbp_platform (Utilities|Casting|CastToBP_Platform OtherActor))
  (for _array_element (Actor|GetComponentsByClass _asbp_platform "/Script/Engine.ActorComponent")
    (if (Utilities|Enum|Equal(Enum) (Utilities|GetObjectName _array_element) "DWallY")
      (CallFunction|DestroyDWallY _asbp_platform))))

(event OnComponentBeginOverlap(LeftPlatfromTriger)
  (params (OverlappedComponent :type Primitive%20Component%20Object%20Reference) (OtherActor :type Actor%20Object%20Reference) (OtherComp :type Primitive%20Component%20Object%20Reference) (OtherBodyIndex :type Integer) (bFromSweep :type Boolean) (SweepResult :type Hit%20Result%20Structure%20%28by%20ref%29))
  ;[0.15 0.15 0.15 0.5] Set platforms link
  (bind _asbp_platform (Utilities|Casting|CastToBP_Platform OtherActor))
  (Variables|Default|SetLeftPlatform _asbp_platform))

(event OnComponentBeginOverlap(RightPlatfromTriger)
  (params (OverlappedComponent :type Primitive%20Component%20Object%20Reference) (OtherActor :type Actor%20Object%20Reference) (OtherComp :type Primitive%20Component%20Object%20Reference) (OtherBodyIndex :type Integer) (bFromSweep :type Boolean) (SweepResult :type Hit%20Result%20Structure%20%28by%20ref%29))
  ;[0.15 0.15 0.15 0.5] Set platforms link
  (bind _asbp_platform (Utilities|Casting|CastToBP_Platform OtherActor)
    (:then
      (Variables|Default|SetRightPlatform _asbp_platform))
    (:CastFailed
      (bind _asbp_platform_admin (Utilities|Casting|CastToBP_PlatformAdmin OtherActor))
      (Variables|Default|SetRightPlatformAdmin _asbp_platform_admin))))

(event Custom|DestroyDoorY
  ;[0.15 0.15 0.15 0.5] Destroy Events
  (Components|DestroyComponent (Variables|Default|GetBP_DoorY)))

(event Custom|DestroyDoorX
  ;[0.15 0.15 0.15 0.5] Destroy Events
  (Components|DestroyComponent (Variables|Default|GetBP_DoorX)))

(event Custom|DestroyDWallY
  ;[0.15 0.15 0.15 0.5] Destroy Events
  (Components|DestroyComponent (Variables|Default|GetDWallY)))

(event Custom|DestroyDWallX
  ;[0.15 0.15 0.15 0.5] Destroy Events
  (Components|DestroyComponent (Variables|Default|GetDWallX)))

(event Custom|SetNewVisibilityWithValidCorection
  (params (Visibility :type Boolean) (Mesh :type Static%20Mesh%20Component%20Object%20Reference))
  ;[0.15 0.15 0.15 0.5] Set visibility
  (Utilities|IsValid Mesh
    (:Is%20Valid
      (Rendering|SetVisibility Mesh Visibility false))))

(event EventBeginPlay
  (bind _self self)
  (bind _self_2 self)
  (bind _defaultsceneroot (Variables|Default|GetDefaultSceneRoot _self))
  (bind _defaultsceneroot_2 (Variables|Default|GetDefaultSceneRoot _self_2))
  (bind _returnvalue (Transformation|GetWorldLocation _defaultsceneroot_2))
  (bind _returnvalue_2 (Transformation|GetWorldLocation _defaultsceneroot))
  (Utilities|FlowControl|Sequence
    (:then_0
      ;[0.15 0.15 0.15 0.5] Cast to BP_SellMachine
      (bind _asbp_sell_machine (Utilities|Casting|CastToBP_SellMachine (Variables|/Script/Engine.ChildActorComponent|GetChildActor (Variables|Default|GetBP_SellMachine))))
      (Variables|Default|SetAs%20BP%20Sell%20Machine _asbp_sell_machine))
    (:then_1
      ;[0.15 0.15 0.15 0.5] Get spawn locaition for room
      (bind _asbp_door (Utilities|Casting|CastToBP_Door (Variables|/Script/Engine.ChildActorComponent|GetChildActor (Variables|Default|GetBP_DoorX))))
      (Variables|/Game/Project/Blueprints/Actors/Locaition/StaticBuyLocaition/BP_Door.BP_Door_C|SetSpawnRoomLocaitain _asbp_door (Math|Vector|MakeVector (- (.x _returnvalue) 8e+02) (.y _returnvalue) (.z _returnvalue))))
    (:then_2
      (bind _asbp_door_2 (Utilities|Casting|CastToBP_Door (Variables|/Script/Engine.ChildActorComponent|GetChildActor (Variables|Default|GetBP_DoorY))))
      (Variables|/Game/Project/Blueprints/Actors/Locaition/StaticBuyLocaition/BP_Door.BP_Door_C|SetSpawnRoomLocaitain _asbp_door_2 (Math|Vector|MakeVector (.x _returnvalue_2) (- (.y _returnvalue_2) 8e+02) (.z _returnvalue_2))))
    (:then_3
      ;[0.15 0.15 0.15 0.5] Set Type Of Locaition
      (Variables|/Game/Project/Blueprints/Actors/Locaition/StaticBuyLocaition/BP_SellMachine.BP_SellMachine_C|SetLocaitionType (Variables|Default|GetAs%20BP%20Sell%20Machine) (Variables|Default|GetLocaition%20Type)))
    (:then_4
      ;[0.15 0.15 0.15 0.5] Set spawn points
      (for (_array_element _array_index) (Variables|Default|GetSpawnPoints)
        (Utilities|Array|Insert (Variables|/Game/Project/Blueprints/Actors/Locaition/StaticBuyLocaition/BP_SellMachine.BP_SellMachine_C|GetState (Variables|Default|GetAs%20BP%20Sell%20Machine)) (Utilities|Struct|MakeS_GamblingMachineStateOnSpawn false (+ (.Location (Math|Transform|BreakTransform _array_element)) (Transformation|GetWorldLocation (Variables|Default|GetDefaultSceneRoot))) (.Rotation (Math|Transform|BreakTransform _array_element))) _array_index)))))

(fn ConstructionScript)