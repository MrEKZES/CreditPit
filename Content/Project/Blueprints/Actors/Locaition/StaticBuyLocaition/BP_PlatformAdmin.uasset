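; BP_PlatformAdmin is a location platform that links a door to the spawn position of an adjacent room.
; On BeginPlay it gives its child BP_Door a room spawn point offset along negative X from its root.
; When its X trigger overlaps a BP_Platform that has a DWallX component, it removes that wall and its own door.
; A player trigger hides the platform's DWallX and DWallY meshes while the character is inside.
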(event OnComponentBeginOverlap(PlayerTrigger)
  (params (OverlappedComponent :type Primitive%20Component%20Object%20Reference) (OtherActor :type Actor%20Object%20Reference) (OtherComp :type Primitive%20Component%20Object%20Reference) (OtherBodyIndex :type Integer) (bFromSweep :type Boolean) (SweepResult :type Hit%20Result%20Structure%20%28by%20ref%29))
  ;[0.15 0.15 0.15 0.5] Player triggers
  (Utilities|Casting|CastToBP_ThirdPersonCharacter OtherActor)
  (CallFunction|SetNewVisibilityforValidCorection false (Variables|Default|GetDWallY))
  (CallFunction|SetNewVisibilityforValidCorection false (Variables|Default|GetDWallX)))

(event OnComponentEndOverlap(PlayerTrigger)
  (params (OverlappedComponent :type Primitive%20Component%20Object%20Reference) (OtherActor :type Actor%20Object%20Reference) (OtherComp :type Primitive%20Component%20Object%20Reference) (OtherBodyIndex :type Integer))
  ;[0.15 0.15 0.15 0.5] Player triggers
  (Utilities|Casting|CastToBP_ThirdPersonCharacter OtherActor)
  (CallFunction|SetNewVisibilityforValidCorection true (Variables|Default|GetDWallY))
  (CallFunction|SetNewVisibilityforValidCorection true (Variables|Default|GetDWallX)))

(event OnComponentBeginOverlap(TriggerDwallX)
  (params (OverlappedComponent :type Primitive%20Component%20Object%20Reference) (OtherActor :type Actor%20Object%20Reference) (OtherComp :type Primitive%20Component%20Object%20Reference) (OtherBodyIndex :type Integer) (bFromSweep :type Boolean) (SweepResult :type Hit%20Result%20Structure%20%28by%20ref%29))
  ;[0.15 0.15 0.15 0.5] Destroy DWalls if room has already created
  (bind _asbp_platform (Utilities|Casting|CastToBP_Platform OtherActor))
  (for _array_element (Actor|GetComponentsByClass _asbp_platform "/Script/Engine.ActorComponent")
    (if (Utilities|Enum|Equal(Enum) (Utilities|GetObjectName _array_element) "DWallX")
      (Default|DestroyDWallX _asbp_platform)
      (Components|DestroyComponent (Variables|Default|GetBP_DoorX)))))

(event Custom|SetNewVisibilityForValidCorection
  (params (Visibility :type Boolean) (Mesh :type Static%20Mesh%20Component%20Object%20Reference))
  ;[0.15 0.15 0.15 0.5] Set visibility
  (Utilities|IsValid Mesh
    (:Is%20Valid
      (Rendering|SetVisibility Mesh Visibility false))))

(event EventBeginPlay
  (bind _self self)
  (bind _defaultsceneroot (Variables|Default|GetDefaultSceneRoot _self))
  (bind _returnvalue (Transformation|GetWorldLocation _defaultsceneroot))
  ;[0.15 0.15 0.15 0.5] Get spawn locaition for room
  (bind _asbp_door (Utilities|Casting|CastToBP_Door (Variables|/Script/Engine.ChildActorComponent|GetChildActor (Variables|Default|GetBP_DoorX))))
  (Variables|/Game/Project/Blueprints/Actors/Locaition/StaticBuyLocaition/BP_Door.BP_Door_C|SetSpawnRoomLocaitain _asbp_door (Math|Vector|MakeVector (- (.x _returnvalue) 8e+02) (.y _returnvalue) (.z _returnvalue))))

(fn ConstructionScript)