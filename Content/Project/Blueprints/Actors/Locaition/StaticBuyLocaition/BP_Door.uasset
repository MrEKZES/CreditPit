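; BP_Door is an interactable door for buying new casino rooms.
; Interacting opens the sell-room widget on the main-level HUD, passing the door itself, and the interact prompt shows only while the HUD allows widget creation.
; SpawnRoom spawns a BP_Platform at the room location, passing the chosen room type and a hardcoded spawn-point layout for Gambling Machine, Poker or Black Jack.
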(event Custom|SpawnRoom
  (params (Locaition%20Type :type E_TypeOfPlatform%20Enum :default "NewEnumerator0"))
  (bind _spawnroomlocaitain (Variables|Default|GetSpawnRoomLocaitain))
  ;[0.15 0.15 0.15 0.5] Spawn BP_Platform
  (switch Utilities|FlowControl|Switch|SwitchonE_TypeOfPlatform Locaition%20Type
    (:NewEnumerator0
      (Game|SpawnActorfromClass "/Game/Project/Blueprints/Actors/Locaition/StaticBuyLocaition/BP_Platform.BP_Platform_C" (Math|Transform|MakeTransform _spawnroomlocaitain "0, 0, 0" "1.000000,1.000000,1.000000") "Undefined" "MultiplyWithRoot" 0 (Utilities|Array|MakeArray (Math|Transform|MakeTransform "150.000000,150.000000,0.000000" "0, 0, 0" "1.000000,1.000000,1.000000") (Math|Transform|MakeTransform "150.000000,-150.000000,0.000000" "0, 0, 0" "1.000000,1.000000,1.000000") (Math|Transform|MakeTransform "-150.000000,150.000000,0.000000" "0, 0, 0" "1.000000,1.000000,1.000000") (Math|Transform|MakeTransform "-150.000000,-150.000000,0.000000" "0, 0, 0" "1.000000,1.000000,1.000000")) Locaition%20Type 0))
    (:NewEnumerator1
      (Game|SpawnActorfromClass "/Game/Project/Blueprints/Actors/Locaition/StaticBuyLocaition/BP_Platform.BP_Platform_C" (Math|Transform|MakeTransform _spawnroomlocaitain "0, 0, 0" "1.000000,1.000000,1.000000") "Undefined" "MultiplyWithRoot" 0 (Utilities|Array|MakeArray (Math|Transform|MakeTransform "0, 0, 0" "0, 0, 0" "1.000000,1.000000,1.000000")) Locaition%20Type 0))
    (:NewEnumerator2
      (Game|SpawnActorfromClass "/Game/Project/Blueprints/Actors/Locaition/StaticBuyLocaition/BP_Platform.BP_Platform_C" (Math|Transform|MakeTransform _spawnroomlocaitain "0, 0, 0" "1.000000,1.000000,1.000000") "Undefined" "MultiplyWithRoot" 0 (Utilities|Array|MakeArray (Math|Transform|MakeTransform "200.000000,0.000000,0.000000" "0, 0, 0" "1.000000,1.000000,1.000000") (Math|Transform|MakeTransform "-200.000000,0.000000,0.000000" "0, 0, 0" "1.000000,1.000000,1.000000")) Locaition%20Type 0))))

(event EventBeginPlay
  ;[0.15 0.15 0.15 0.5] Cast to HUD
  (bind _asbp_hudmain_levels (Utilities|Casting|CastToBP_HUDMainLevels (HUD|GetHUD (Game|GetPlayerController 0))))
  (Variables|Default|SetAs%20BP%20HUDMain%20Levels _asbp_hudmain_levels))

(event EventInteract
  ;[0.15 0.15 0.15 0.5] Interact
  (Default|AddWBPSellRoom (Variables|Default|GetAs%20BP%20HUDMain%20Levels) self))

(fn ConstructionScript)

(fn PreInteract
  (if (Variables|/Game/Project/Blueprints/UI/HUDs/MainLevels/BP_HUDMainLevels.BP_HUDMainLevels_C|GetbWidgetMayBeCreate (Variables|Default|GetAs%20BP%20HUDMain%20Levels))
    (return "Press E to interact")
    (else
      (return ""))))