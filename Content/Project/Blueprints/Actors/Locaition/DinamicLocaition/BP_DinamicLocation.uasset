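; Actor Blueprint that procedurally builds a simple room or arena location from cube meshes.
; The Construction Script calls AddFloor, which adds a scaled floor with a configurable material, then AddWalls, which adds four perimeter walls.
; Wall scale and offsets derive from the floor's world scale, wall thickness and height, assuming a 100-unit cube, so walls sit flush on the floor's edges.
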(event Custom|AddFloor
  ;[0.15 0.15 0.15 0.5] Add Floor (Static Mesh Component)
  (bind _returnvalue (AddComponent|AddStaticMeshComponent false))
  (bind _output_get (Variables|FloorComponent|SetFloor _returnvalue))
  (Components|StaticMesh|SetStaticMesh _output_get "/Engine/BasicShapes/Cube.Cube")
  ;[0.15 0.15 0.15 0.5] Set Floor Scale
  (Transformation|SetRelativeScale3D (Variables|FloorComponent|GetFloor) (Variables|FloorComponent|GetFloorScale))
  ;[0.15 0.15 0.15 0.5] Set Floor Material
  (Rendering|Material|SetMaterial (Variables|FloorComponent|GetFloor) 0 (Variables|FloorComponent|GetFloorMaterial)))

(event Custom|AddWalls
  (bind _floor (Variables|FloorComponent|GetFloor))
  (bind _floor_2 (Variables|FloorComponent|GetFloor))
  (bind _floor_3 (Variables|FloorComponent|GetFloor))
  (bind _floor_4 (Variables|FloorComponent|GetFloor))
  (bind _returnvalue (Transformation|GetWorldScale _floor))
  (bind _returnvalue_2 (Transformation|GetWorldScale _floor_2))
  (bind _returnvalue_3 (Transformation|GetWorldScale _floor_3))
  (bind _returnvalue_4 (Transformation|GetWorldScale _floor_4))
  (Utilities|FlowControl|Sequence
    (:then_0
      ;[0.15 0.15 0.15 0.5] Add Wall (Static Mesh Component)
      (bind _returnvalue_5 (AddComponent|AddStaticMeshComponent false))
      (bind _output_get (Variables|WallComponent|SetWall _returnvalue_5))
      (Components|StaticMesh|SetStaticMesh _output_get "/Engine/BasicShapes/Cube.Cube")
      ;[0.15 0.15 0.15 0.5] Set Wall Scale
      (Transformation|SetRelativeScale3D (Variables|WallComponent|GetWall) (Math|Vector|MakeVector (Variables|WallComponent|GetWallThickness) (.y (Transformation|GetWorldScale (Variables|FloorComponent|GetFloor))) (Variables|WallComponent|GetWallHeight)))
      ;[0.15 0.15 0.15 0.5] Set Wall Locaition on the Floor surface
      (Transformation|AddLocalOffset (Variables|WallComponent|GetWall) (Math|Vector|MakeVector (- (* (.x _returnvalue_2) 50) (* (Variables|WallComponent|GetWallThickness) 50)) 0.0 (+ (* (Variables|WallComponent|GetWallHeight) 50) (* (.z _returnvalue_2) 50))) false false))
    (:then_1
      ;[0.15 0.15 0.15 0.5] Add Wall (Static Mesh Component)
      (bind _returnvalue_6 (AddComponent|AddStaticMeshComponent false))
      (bind _output_get_2 (Variables|WallComponent|SetWall _returnvalue_6))
      (Components|StaticMesh|SetStaticMesh _output_get_2 "/Engine/BasicShapes/Cube.Cube")
      ;[0.15 0.15 0.15 0.5] Set Wall Scale
      (Transformation|SetRelativeScale3D (Variables|WallComponent|GetWall) (Math|Vector|MakeVector (Variables|WallComponent|GetWallThickness) (.y (Transformation|GetWorldScale (Variables|FloorComponent|GetFloor))) (Variables|WallComponent|GetWallHeight)))
      ;[0.15 0.15 0.15 0.5] Set Wall Locaition on the Floor surface
      (Transformation|AddLocalOffset (Variables|WallComponent|GetWall) (Math|Vector|MakeVector (- (* (.x _returnvalue_3) -50) (* (Variables|WallComponent|GetWallThickness) -50)) 0.0 (+ (* (Variables|WallComponent|GetWallHeight) 50) (* (.z _returnvalue_3) 50))) false false))
    (:then_2
      ;[0.15 0.15 0.15 0.5] Add Wall (Static Mesh Component)
      (bind _returnvalue_7 (AddComponent|AddStaticMeshComponent false))
      (bind _output_get_3 (Variables|WallComponent|SetWall _returnvalue_7))
      (Components|StaticMesh|SetStaticMesh _output_get_3 "/Engine/BasicShapes/Cube.Cube")
      ;[0.15 0.15 0.15 0.5] Set Wall Scale
      (Transformation|SetRelativeScale3D (Variables|WallComponent|GetWall) (Math|Vector|MakeVector (.x (Transformation|GetWorldScale (Variables|FloorComponent|GetFloor))) (Variables|WallComponent|GetWallThickness) (Variables|WallComponent|GetWallHeight)))
      ;[0.15 0.15 0.15 0.5] Set Wall Locaition on the Floor surface
      (Transformation|AddLocalOffset (Variables|WallComponent|GetWall) (Math|Vector|MakeVector 0.0 (- (* (.y _returnvalue_4) -50) (* (Variables|WallComponent|GetWallThickness) -50)) (+ (* (Variables|WallComponent|GetWallHeight) 50) (* (.z _returnvalue_4) 50))) false false))
    (:then_3
      ;[0.15 0.15 0.15 0.5] Add Wall (Static Mesh Component)
      (bind _returnvalue_8 (AddComponent|AddStaticMeshComponent false))
      (bind _output_get_4 (Variables|WallComponent|SetWall _returnvalue_8))
      (Components|StaticMesh|SetStaticMesh _output_get_4 "/Engine/BasicShapes/Cube.Cube")
      ;[0.15 0.15 0.15 0.5] Set Wall Scale
      (Transformation|SetRelativeScale3D (Variables|WallComponent|GetWall) (Math|Vector|MakeVector (.x (Transformation|GetWorldScale (Variables|FloorComponent|GetFloor))) (Variables|WallComponent|GetWallThickness) (Variables|WallComponent|GetWallHeight)))
      ;[0.15 0.15 0.15 0.5] Set Wall Locaition on the Floor surface
      (Transformation|AddLocalOffset (Variables|WallComponent|GetWall) (Math|Vector|MakeVector 0.0 (- (* (.y _returnvalue) 50) (* (Variables|WallComponent|GetWallThickness) 50)) (+ (* (Variables|WallComponent|GetWallHeight) 50) (* (.z _returnvalue) 50))) false false))))

(fn ConstructionScript
  (CallFunction|AddFloor)
  (CallFunction|AddWalls))