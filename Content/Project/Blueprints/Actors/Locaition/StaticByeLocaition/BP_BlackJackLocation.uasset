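; Blackjack room actor that acts as an expandable location tile, with doors toward neighbouring rooms and a sell machine.
; BeginPlay gives both doors room spawn positions offset along -X and -Y, then passes the machine a spawn slot and location type.
; Player overlap hides dynamic walls, while adjoining gambling-machine rooms hide static walls.
; An overlapping blackjack room has its X door destroyed; the matching Y logic is disconnected.
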(event OnComponentBeginOverlap(PlayerTrigger)
  (params (OverlappedComponent :type Primitive%20Component%20Object%20Reference) (OtherActor :type Actor%20Object%20Reference) (OtherComp :type Primitive%20Component%20Object%20Reference) (OtherBodyIndex :type Integer) (bFromSweep :type Boolean) (SweepResult :type Hit%20Result%20Structure%20%28by%20ref%29))
  ;[0.15 0.15 0.15 0.5] Set Visibility DinamicWall
  (Utilities|Casting|CastToBP_ThirdPersonCharacter OtherActor)
  (Rendering|SetVisibility (Variables|Default|GetDWallY) false false))

(event OnComponentEndOverlap(PlayerTrigger)
  (params (OverlappedComponent :type Primitive%20Component%20Object%20Reference) (OtherActor :type Actor%20Object%20Reference) (OtherComp :type Primitive%20Component%20Object%20Reference) (OtherBodyIndex :type Integer))
  ;[0.15 0.15 0.15 0.5] Set Visibility DinamicWall
  (Utilities|Casting|CastToBP_ThirdPersonCharacter OtherActor)
  (Rendering|SetVisibility (Variables|Default|GetDWallY) true false))

(event OnComponentBeginOverlap(OtherLocaitionTriggetX)
  (params (OverlappedComponent :type Primitive%20Component%20Object%20Reference) (OtherActor :type Actor%20Object%20Reference) (OtherComp :type Primitive%20Component%20Object%20Reference) (OtherBodyIndex :type Integer) (bFromSweep :type Boolean) (SweepResult :type Hit%20Result%20Structure%20%28by%20ref%29))
  ;[0.15 0.15 0.15 0.5] Set Visibility StaticWall
  (Utilities|Casting|CastToBP_GamblingMachineLocation OtherActor)
  (Rendering|SetVisibility (Variables|Default|GetWallX) false false))

(event OnComponentBeginOverlap(OtherLocaitionTriggetY)
  (params (OverlappedComponent :type Primitive%20Component%20Object%20Reference) (OtherActor :type Actor%20Object%20Reference) (OtherComp :type Primitive%20Component%20Object%20Reference) (OtherBodyIndex :type Integer) (bFromSweep :type Boolean) (SweepResult :type Hit%20Result%20Structure%20%28by%20ref%29))
  ;[0.15 0.15 0.15 0.5] Set Visibility StaticWall
  (Utilities|Casting|CastToBP_GamblingMachineLocation OtherActor)
  (Rendering|SetVisibility (Variables|Default|GetWallY) false false))

(event OnComponentBeginOverlap(TriggerDoorX)
  (params (OverlappedComponent :type Primitive%20Component%20Object%20Reference) (OtherActor :type Actor%20Object%20Reference) (OtherComp :type Primitive%20Component%20Object%20Reference) (OtherBodyIndex :type Integer) (bFromSweep :type Boolean) (SweepResult :type Hit%20Result%20Structure%20%28by%20ref%29))
  ;[0.15 0.15 0.15 0.5] Destroy Door system if room has already been created
  (bind _asbp_black_jack_machine_location (Utilities|Casting|CastToBP_BlackJackLocation OtherActor))
  (for _array_element (Actor|GetComponentsByClass _asbp_black_jack_machine_location "/Script/Engine.ActorComponent")
    (if (Utilities|Enum|Equal(Enum) (Utilities|GetObjectName _array_element) "BP_DoorX")
      (CallFunction|DestroyDoorX _asbp_black_jack_machine_location))))

(event OnComponentBeginOverlap(TriggerDoorY)
  (params (OverlappedComponent :type Primitive%20Component%20Object%20Reference) (OtherActor :type Actor%20Object%20Reference) (OtherComp :type Primitive%20Component%20Object%20Reference) (OtherBodyIndex :type Integer) (bFromSweep :type Boolean) (SweepResult :type Hit%20Result%20Structure%20%28by%20ref%29))
  ;[0.15 0.15 0.15 0.5] Destroy Door system if room has already been created
  (bind _asbp_black_jack_machine_location (Utilities|Casting|CastToBP_BlackJackLocation OtherActor)))

(event Custom|DestroyDoorY
  ;[0.15 0.15 0.15 0.5] Destroy Events
  (Components|DestroyComponent (Variables|Default|GetBP_DoorY)))

(event Custom|DestroyDoorX
  ;[0.15 0.15 0.15 0.5] Destroy Events
  (Components|DestroyComponent (Variables|Default|GetBP_DoorX)))

(event EventBeginPlay
  (bind _self self)
  (bind _self_2 self)
  (bind _spawnpoint1position (Variables|Default|GetSpawnPoint1Position))
  (bind _returnvalue (Transformation|GetWorldTransform _spawnpoint1position))
  (bind _defaultsceneroot (Variables|Default|GetDefaultSceneRoot _self))
  (bind _defaultsceneroot_2 (Variables|Default|GetDefaultSceneRoot _self_2))
  (bind _returnvalue_2 (Transformation|GetWorldLocation _defaultsceneroot_2))
  (bind _returnvalue_3 (Transformation|GetWorldLocation _defaultsceneroot))
  (Utilities|FlowControl|Sequence
    (:then_0
      ;[0.15 0.15 0.15 0.5] Get spawn locaition for room
      (bind _asbp_door (Utilities|Casting|CastToBP_Door (Variables|/Script/Engine.ChildActorComponent|GetChildActor (Variables|Default|GetBP_DoorX))))
      (Variables|/Game/Project/Blueprints/Actors/Locaition/StaticByeLocaition/BP_Door.BP_Door_C|SetSpawnRoomLocaitain _asbp_door (Math|Vector|MakeVector (- (.x _returnvalue_2) 8e+02) (.y _returnvalue_2) (.z _returnvalue_2)))
      ;[0.15 0.15 0.15 0.5] get spawn locaition for black jack
      (bind _asbp_sell_machine (Utilities|Casting|CastToBP_SellMachine (Variables|/Script/Engine.ChildActorComponent|GetChildActor (Variables|Default|GetBP_SellMachine))))
      (Variables|Default|SetAs%20BP%20Sell%20Machine _asbp_sell_machine)
      (Utilities|Array|Insert (Variables|/Game/Project/Blueprints/Actors/Locaition/StaticByeLocaition/BP_SellMachine.BP_SellMachine_C|GetState (Variables|Default|GetAs%20BP%20Sell%20Machine)) (Utilities|Struct|MakeS_GamblingMachineStateOnSpawn false (.location _returnvalue) (.rotation _returnvalue)))
      (Components|DestroyComponent (Variables|Default|GetSpawnPoint1Position)))
    (:then_1
      (bind _asbp_door_2 (Utilities|Casting|CastToBP_Door (Variables|/Script/Engine.ChildActorComponent|GetChildActor (Variables|Default|GetBP_DoorY))))
      (Variables|/Game/Project/Blueprints/Actors/Locaition/StaticByeLocaition/BP_Door.BP_Door_C|SetSpawnRoomLocaitain _asbp_door_2 (Math|Vector|MakeVector (.x _returnvalue_3) (- (.y _returnvalue_3) 8e+02) (.z _returnvalue_3))))
    (:then_2
      ;[0.15 0.15 0.15 0.5] Set Type Of Locaition
      (Variables|/Game/Project/Blueprints/Actors/Locaition/StaticByeLocaition/BP_SellMachine.BP_SellMachine_C|SetLocaitionTipe (Variables|Default|GetAs%20BP%20Sell%20Machine) "NewEnumerator2"))))

(fn ConstructionScript)