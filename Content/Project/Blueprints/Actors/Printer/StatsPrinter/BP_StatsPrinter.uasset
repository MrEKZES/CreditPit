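; BP_StatsPrinter is a debug actor that prints player stats on screen every frame.
; On BeginPlay it casts the player pawn to BP_ThirdPersonCharacter and caches it.
; Tick formats the money and oligarch-mode flag from that character's BPMoneySystem, plus FPS derived from delta time.
; The EXP and Level fields show a literal ERROR placeholder rather than real values.
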(event EventBeginPlay
  (bind _asbp_third_person_character (Utilities|Casting|CastToBP_ThirdPersonCharacter (Game|Player|GetPlayerPawn 0)))
  (Variables|Default|SetAs%20BP%20Third%20Person%20Character _asbp_third_person_character))

(event EventTick
  (params (DeltaSeconds :type Float%20%28single-precision%29))
  (bind _as_bp_third_person_character (Variables|Default|GetAs%20BP%20Third%20Person%20Character))
  (bind _bp_moneysystem (Variables|/Game/ThirdPerson/Blueprints/BP_ThirdPersonCharacter.BP_ThirdPersonCharacter_C|GetBP_MoneySystem _as_bp_third_person_character))
  (Development|PrintText (Utilities|Text|FormatText "Money: {money} 
Gog mode: {godMode} 
EXP: ERROR 
Level: ERROR 
FPS: {fps} 
" (Variables|/Game/Project/Blueprints/Components/BP_MoneySystem.BP_MoneySystem_C|GetMoney _bp_moneysystem) (Variables|/Game/Project/Blueprints/Components/BP_MoneySystem.BP_MoneySystem_C|GetbInOligarchMod _bp_moneysystem) (/ 1.0 DeltaSeconds)) true false "(R=1.000000,G=0.000000,B=0.000000,A=1.000000)" 0.0))

(fn ConstructionScript)