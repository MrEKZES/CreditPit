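; BP_NPCManager is an NPC spawner that periodically creates BP_NPC actors and sends them to gambling machines.
; On BeginPlay it starts a looping timer whose interval is picked once at random between the min and max spawner range.
; Each tick of the timer spawns an NPC at the manager's transform, then moves it to the socket point of the first machine in GamblingMachines with available seats, if any.
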(event Custom|Create%20NPC
  (bind _returnvalue (Game|SpawnActorfromClass "/Game/Project/Blueprints/Actors/NPC/BP_NPC.BP_NPC_C" (Transformation|GetActorTransform self) "Undefined" "MultiplyWithRoot" 0 0))
  (bind _array_element (Utilities|Array|ForEachLoopwithBreak (Variables|Default|GetGamblingMachines) :!label _label)
    (:LoopBody
      (if (> (Variables|/Game/Project/Blueprints/Actors/Machines/BP_GamblingBaseActor.BP_GamblingBaseActor_C|GetAvailableSeats _array_element) 0)
        (Utilities|FlowControl|Sequence
          (:then_0
            (Default|Moveto _returnvalue (Transformation|GetWorldLocation (Variables|/Game/Project/Blueprints/Actors/Machines/BP_GamblingBaseActor.BP_GamblingBaseActor_C|GetSocketPoint _array_element))))
          (:then_1
            (goto _label Break)))))))

(event EventBeginPlay
  (Utilities|Time|SetTimerbyEvent (delegate Custom|Create%20NPC) (Math|Random|RandomFloatinRange (Variables|Default|GetMinSpawnerRange) (Variables|Default|GetMaxSpawnerRange)) true))

(fn ConstructionScript)