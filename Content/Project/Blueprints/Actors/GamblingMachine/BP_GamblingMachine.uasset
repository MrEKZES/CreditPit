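; Gambling machine actor that feeds money to the player's BPMoneySystem as NPCs play it, and can be upgraded by interacting.
; An NPC entering the box marks it busy and triggers delayed payments from that NPC's roll count and bet, alongside a temporary looping money timer.
; Upgrades raise level and MoneyPerRoll before the money check, then swap the mesh by level tier on success; payouts ignore MoneyPerRoll.
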(event OnComponentBeginOverlap(Box)
  (params (OverlappedComponent :type Primitive%20Component%20Object%20Reference) (OtherActor :type Actor%20Object%20Reference) (OtherComp :type Primitive%20Component%20Object%20Reference) (OtherBodyIndex :type Integer) (bFromSweep :type Boolean) (SweepResult :type Hit%20Result%20Structure%20%28by%20ref%29))
  (bind _asbp_npc (Utilities|Casting|CastToBP_NPC OtherActor))
  (bind _output_get (Variables|Default|SetAs%20BP%20NPC _asbp_npc))
  (Variables|GamblingMachine|SetbIsBusy true)
  (for _index (range 0 (Variables|/Game/Project/Blueprints/Actors/NPC/BP_NPC.BP_NPC_C|GetRollCount _output_get))
    (Utilities|FlowControl|Delay (Variables|GamblingMachine|GetTimeBetwenRoll))
    (Default|InteractwithMoney (Variables|/Game/ThirdPerson/Blueprints/BP_ThirdPersonCharacter.BP_ThirdPersonCharacter_C|GetBP_MoneySystem (Variables|Default|GetAs%20BP_ThirdPersonCharacter)) "NewEnumerator0" (Variables|/Game/Project/Blueprints/Actors/NPC/BP_NPC.BP_NPC_C|GetBetSum _output_get))))

(event OnComponentEndOverlap(Box)
  (params (OverlappedComponent :type Primitive%20Component%20Object%20Reference) (OtherActor :type Actor%20Object%20Reference) (OtherComp :type Primitive%20Component%20Object%20Reference) (OtherBodyIndex :type Integer))
  (Variables|GamblingMachine|SetbIsBusy false))

(event Custom|GM%20Upgrade
  (bind _level (Variables|GamblingMachine|GetLevel))
  (bind _cube (Variables|Default|GetCube))
  (Math|Integer|IncrementInt (Variables|GamblingMachine|GetLevel)
    (:%20%20
      (Variables|GamblingMachine|SetMoneyPerRoll (+ (Variables|GamblingMachine|GetMoneyPerRoll) 100))
      (bind _actioniscomplited (Default|InteractwithMoney (Variables|/Game/ThirdPerson/Blueprints/BP_ThirdPersonCharacter.BP_ThirdPersonCharacter_C|GetBP_MoneySystem (Variables|Default|GetAs%20BP_ThirdPersonCharacter)) "NewEnumerator1" 100))
      (if _actioniscomplited
        (Development|PrintString (Utilities|String|ToString(Integer) _level))
        (switch int (/ _level 25)
          (:1
            (Components|StaticMesh|SetStaticMesh _cube "/Game/Project/Models/GamblingMachine/mashine1_test.mashine1_test"))
          (:2
            (Components|StaticMesh|SetStaticMesh _cube "/Game/Project/Models/GamblingMachine/mashine2_test.mashine2_test"))
          (:3
            (Components|StaticMesh|SetStaticMesh _cube 0))
          (:4
            (Components|StaticMesh|SetStaticMesh _cube 0)))))))

(event Custom|1
  ;[1 0 0] VREMENNO
  (Default|InteractwithMoney (Variables|/Game/ThirdPerson/Blueprints/BP_ThirdPersonCharacter.BP_ThirdPersonCharacter_C|GetBP_MoneySystem (Variables|Default|GetAs%20BP_ThirdPersonCharacter)) "NewEnumerator0" 5))

(event EventInteractE
  (CallFunction|GMUpgrade))

(event EventBeginPlay
  (Utilities|Time|SetTimerbyEvent (delegate Custom|1) 0.5 true))

(fn ConstructionScript)