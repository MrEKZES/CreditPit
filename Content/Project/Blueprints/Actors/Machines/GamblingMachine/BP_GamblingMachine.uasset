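; Interactable gambling machine actor that exchanges money with the player's BPMoneySystem and can be upgraded through levels.
; A looping timer started on BeginPlay makes a fixed money transaction, independent of MoneyPerRoll.
; Interact calls Upgrade, which raises Level and MoneyPerRoll before attempting a separate transaction, even if that transaction fails.
; A successful transaction prints the level and swaps the cube's mesh from the LevelMeshes map.
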(event Custom|Upgrade
  (bind _level (Variables|GamblingMachine|GetLevel))
  (bind _levelmeshes (Variables|Default|GetLevelMeshes))
  (bind (_value _returnvalue) (Utilities|Map|Find _levelmeshes _level))
  (Math|Integer|IncrementInt (Variables|GamblingMachine|GetLevel)
    (:%20%20
      (Variables|GamblingMachine|SetMoneyPerRoll (+ (Variables|GamblingMachine|GetMoneyPerRoll) 100))
      (bind _actioniscomplited (Default|InteractwithMoney (Variables|/Game/ThirdPerson/Blueprints/BP_ThirdPersonCharacter.BP_ThirdPersonCharacter_C|GetBP_MoneySystem (Variables|Default|GetAs%20BP_ThirdPersonCharacter)) "NewEnumerator1" 100))
      (if _actioniscomplited
        (Development|PrintString (Utilities|String|ToString(Integer) _level))
        (if _returnvalue
          (Components|StaticMesh|SetStaticMesh (Variables|Default|GetCube) _value))))))

(event Custom|1
  (Default|InteractwithMoney (Variables|/Game/ThirdPerson/Blueprints/BP_ThirdPersonCharacter.BP_ThirdPersonCharacter_C|GetBP_MoneySystem (Variables|Default|GetAs%20BP_ThirdPersonCharacter)) "NewEnumerator0" 5))

(event EventInteract
  (CallFunction|Upgrade))

(event EventBeginPlay
  (Utilities|Time|SetTimerbyEvent (delegate Custom|1) 0.5 true))

(fn ConstructionScript)

(fn PreInteract
  (return ""))