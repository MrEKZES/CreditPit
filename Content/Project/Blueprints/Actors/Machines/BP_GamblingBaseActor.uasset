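; Base actor for an upgradeable gambling machine that earns the player passive money from seated NPCs.
; It registers with BP_NPCManager, tracks free seats, and runs a looping timer that pays level income per occupied seat.
; Robber NPCs deduct that income instead, and a rare jackpot deducts a large payout with animation and sound.
; Interacting buys the next GLData level, swapping the mesh and refreshing the HUD prompt.
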(event Custom|TakeASeat
  (Math|Integer|DecrementInt (Variables|Default|GetAvailableSeats)))

(event Custom|Upgrade
  (if (< (Variables|Default|GetLevel) (Utilities|Array|LastIndex (Variables|Default|GetGLData)))
    (bind _actioniscomplited (Default|InteractwithMoney (Variables|/Game/ThirdPerson/Blueprints/BP_ThirdPersonCharacter.BP_ThirdPersonCharacter_C|GetBP_MoneySystem (Variables|Default|GetAs%20BP%20Third%20Person%20Character)) "NewEnumerator1" (.moneytolvl (Utilities|Array|Get(acopy) (Variables|Default|GetGLData) (Variables|Default|GetLevel)))))
    (if _actioniscomplited
      (Math|Integer|IncrementInt (Variables|Default|GetLevel)
        (:%20%20
          (Components|StaticMesh|SetStaticMesh (Variables|Default|GetMainMesh) (.levelmesh (Utilities|Array|Get(acopy) (Variables|Default|GetGLData) (Variables|Default|GetLevel))))
          (Audio|PlaySound2D "/Game/Project/MaterialLibrary/Sounds/Buy2.Buy2" 1.0 1.0 0.0 0 0))))))

(event Custom|CreatPassiveMoneyIncome
  (Utilities|Time|SetTimerbyEvent (delegate Custom|IncomeTimer) (Variables|Default|GetTickInterval) true))

(event Custom|IncomeTimer
  (bind _npc (Variables|Default|GetNPC))
  (bind _mesh (Variables|/Script/Engine.Character|GetMesh _npc))
  (Utilities|IsValid (Variables|Default|GetNPC)
    (:Is%20Valid
      (if (Variables|/Game/Project/Blueprints/Actors/NPC/BP_NPC.BP_NPC_C|GetbRobber (Variables|Default|GetNPC))
        ;[0.15 0.15 0.15 0.5] Shuler substr
        (Default|InteractwithMoney (Variables|/Game/ThirdPerson/Blueprints/BP_ThirdPersonCharacter.BP_ThirdPersonCharacter_C|GetBP_MoneySystem (Variables|Default|GetAs%20BP%20Third%20Person%20Character)) "NewEnumerator2" (* (.lvlincome (Utilities|Array|Get(acopy) (Variables|Default|GetGLData) (Variables|Default|GetLevel))) (- (Variables|Default|GetMaxSeats) (Variables|Default|GetAvailableSeats))))
        (elif (== (Math|Random|RandomIntegerinRange 0 200) 5)
          ;[0.15 0.15 0.15 0.5] JackPot
          (Default|InteractwithMoney (Variables|/Game/ThirdPerson/Blueprints/BP_ThirdPersonCharacter.BP_ThirdPersonCharacter_C|GetBP_MoneySystem (Variables|Default|GetAs%20BP%20Third%20Person%20Character)) "NewEnumerator2" (* (.lvlincome (Utilities|Array|Get(acopy) (Variables|Default|GetGLData) (Variables|Default|GetLevel))) 100))
          (Components|Animation|PlayAnimation _mesh "/Game/Project/Models/NPC/Jackpot.Jackpot" false)
          (Audio|PlaySound2D "/Game/Project/MaterialLibrary/Sounds/Jackpot.Jackpot" 1.0 1.0 0.0 0 0)
          (Utilities|FlowControl|Delay 1.0)
          (Components|Animation|PlayAnimation _mesh "/Game/Project/Models/NPC/Idle.Idle" true)
          (else
            ;[0.15 0.15 0.15 0.5] Add
            (Default|InteractwithMoney (Variables|/Game/ThirdPerson/Blueprints/BP_ThirdPersonCharacter.BP_ThirdPersonCharacter_C|GetBP_MoneySystem (Variables|Default|GetAs%20BP%20Third%20Person%20Character)) "NewEnumerator0" (* (.lvlincome (Utilities|Array|Get(acopy) (Variables|Default|GetGLData) (Variables|Default|GetLevel))) (- (Variables|Default|GetMaxSeats) (Variables|Default|GetAvailableSeats))))))))))

(event Custom|FreeUpSeat
  (Math|Integer|IncrementInt (Variables|Default|GetAvailableSeats)))

(event EventBeginPlay
  (CallFunction|CreatPassiveMoneyIncome)
  (bind _returnvalue (Actor|GetActorOfClass "/Game/Project/Blueprints/Actors/NPC/BP_NPCManager.BP_NPCManager_C"))
  (Utilities|Array|Add (Variables|/Game/Project/Blueprints/Actors/NPC/BP_NPCManager.BP_NPCManager_C|GetGamblingMachines _returnvalue) self)
  (Variables|Default|SetMaxSeats (Variables|Default|GetAvailableSeats))
  (Rendering|Material|SetMaterial (Variables|Default|GetMainMesh) 0 0)
  (Components|StaticMesh|SetStaticMesh (Variables|Default|GetMainMesh) (.levelmesh (Utilities|Array|Get(acopy) (Variables|Default|GetGLData)))))

(event EventInteract
  (CallFunction|Upgrade)
  (bind _outtext (CallFunction|PreInteract))
  (Variables|/Game/Project/Blueprints/UI/Widgets/MainLevels/WBP_ObjectInteractable.WBP_ObjectInteractable_C|SetOutText (Variables|/Game/Project/Blueprints/UI/HUDs/MainLevels/BP_HUDMainLevels.BP_HUDMainLevels_C|GetWBP_ObjectInteractable (Variables|/Game/ThirdPerson/Blueprints/BP_ThirdPersonCharacter.BP_ThirdPersonCharacter_C|GetAs%20BP%20HUDMain%20Levels (Variables|Default|GetAs%20BP%20Third%20Person%20Character))) _outtext))

(fn ConstructionScript)

(fn PreInteract
  (if (< (Variables|Default|GetLevel) (Utilities|Array|LastIndex (Variables|Default|GetGLData)))
    (return (Utilities|Text|FormatText "Press E to upgrade. Upgrade cost: {moneyToUpgrade}" (.moneytolvl (Utilities|Array|Get(acopy) (Variables|Default|GetGLData) (Variables|Default|GetLevel)))))
    (else
      (return "MAX"))))