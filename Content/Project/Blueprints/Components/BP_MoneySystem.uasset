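; BP_MoneySystem is a money component that adds to or subtracts from a Money value through an InteractWithMoney event.
; An oligarch mode flag starts off on BeginPlay and toggles with the L key.
; While the mode is on, InteractWithMoney leaves the balance untouched.
; Tick prints the flag's state every frame as debug output.
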(event Custom|InteractWithMoney
  (params (Interact :type E_InteractWithMoney%20Enum :default "NewEnumerator0") (Money :type Integer))
  (if (not (Variables|Default|GetbInOligarchMod))
    (switch Utilities|FlowControl|Switch|SwitchonE_InteractWithMoney Interact
      (:NewEnumerator0
        (Variables|Default|SetMoney (+ Money (Variables|Default|GetMoney))))
      (:NewEnumerator1
        (Variables|Default|SetMoney (- (Variables|Default|GetMoney) Money))))))

(event EventBeginPlay
  ;[0.15 0.15 0.15 0.5] Set oligarh mod
  (Variables|Default|SetbInOligarchMod false))

(event EventTick
  (params (DeltaSeconds :type Float%20%28single-precision%29))
  (bind _binoligarchmod (Variables|Default|GetbInOligarchMod))
  (bind _returnvalue (Utilities|String|ToString(Boolean) _binoligarchmod))
  ;[0.15 0.15 0.15 0.5] Print oligarh mod
  (if _binoligarchmod
    (Development|PrintString _returnvalue true true "(R=0.000000,G=1.000000,B=0.000000,A=1.000000)" 0.0)
    (else
      (Development|PrintString _returnvalue true true "(R=1.000000,G=0.000000,B=0.000000,A=1.000000)" 0.0))))

(event Input|KeyboardEvents|L
  (params (Key :type Key%20Structure :default "None"))
  ;[0.15 0.15 0.15 0.5] Set oligarh mod to buttons
  (:Pressed
    (Variables|Default|SetbInOligarchMod (not (Variables|Default|GetbInOligarchMod)))))